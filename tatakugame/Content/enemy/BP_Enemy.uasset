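; BP_Enemy is an enemy actor that flips its rotation on collision and can be killed by damage.
; A capsule hit combines the actor's current rotation with a 180-degree offset on one axis.
; AnyDamage subtracts the damage from HPEnemy and prints the remaining value.
; When HP drops below 1, it prints a death message and destroys the actor.
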(event `self.CapsuleComponent.OnComponentHit`
  (params (HitComponent :type "PrimitiveComponent Object Reference") (OtherActor :type "Actor Object Reference") (OtherComp :type "PrimitiveComponent Object Reference") (NormalImpulse :type "Vector Structure") (Hit :type "HitResult Structure (by ref)"))
  (`self.K2_SetActorRotation` (`KismetMathLibrary.ComposeRotators` (`self.K2_GetActorRotation`) (struct :`Yaw` 180.0))))

(event `self.ReceiveAnyDamage`
  (params (Damage :type "Float (single-precision)") (DamageType :type "DamageType Object Reference") (InstigatedBy :type "Controller Object Reference") (DamageCauser :type "Actor Object Reference"))
  (bind _output_get (set `self.HP_Enemy` (- (`self.HP_Enemy`) Damage))) ; セットは値を記憶できる
  (`KismetSystemLibrary.PrintString` (`KismetStringLibrary.Conv_DoubleToString` _output_get))
  (if (< _output_get 1.0)
    (`KismetSystemLibrary.PrintString` "死亡")
    (`self.K2_DestroyActor`)))

(fn `UserConstructionScript`)